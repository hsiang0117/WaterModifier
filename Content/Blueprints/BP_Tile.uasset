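; BP_Tile is a map tile actor that shows an imported image on one Paper sprite and a water mask overlay on a second.
; SetTexture loads a file into a dynamic instance of M_BaseMaterial, destroying the tile if the import fails.
; SetWatermask lazily builds the mask texture from a file, caching success or failure in flags so later calls only toggle visibility.
; RefreshWatermask rebuilds the mask regardless of those flags, and HideWatermask hides it.
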(event EventBeginPlay)

(event Collision|EventActorBeginOverlap
  (params (OtherActor :type Actor%20Object%20Reference)))

(event EventTick
  (params (DeltaSeconds :type Float%20%28single-precision%29)))

(fn ConstructionScript)

(fn SetTexture
  (params (FilePath :type String))
  (bind _returnvalue (Class|MyBlueprintFunctionLibrary|MyImportFileasTexture2D FilePath))
  (Utilities|IsValid _returnvalue
    (:Is%20Valid
      (bind _returnvalue_2 (Rendering|Material|CreateDynamicMaterialInstance "/Game/Materials/M_BaseMaterial.M_BaseMaterial" "None" "Transient" :!class /Script/Engine.KismetMaterialLibrary))
      (Rendering|Material|SetTextureParameterValue _returnvalue_2 "Texture" _returnvalue)
      (Rendering|Material|SetMaterial (Variables|Default|GetMapPaperSprite) 0 _returnvalue_2))
    (:Is%20Not%20Valid
      (Actor|DestroyActor))))

(fn SetWatermask
  (params (FilePath :type String) (TileSize :type Integer))
  (bind _waterpapersprite (Variables|Default|GetWaterPaperSprite))
  (if (Variables|Default|GetWatermaskLoaded)
    (Rendering|SetVisibility (Variables|Default|GetWaterPaperSprite) true false)
    (elif (not (Variables|Default|GetWatermaskInvalid))
      (bind _returnvalue (Class|MyBlueprintFunctionLibrary|CreateTexturefromWatermaskArray FilePath TileSize))
      (Utilities|IsValid _returnvalue
        (:Is%20Valid
          (bind _returnvalue_2 (Rendering|Material|CreateDynamicMaterialInstance "/Game/Materials/M_BaseMaterial.M_BaseMaterial" "None" "Transient" :!class /Script/Engine.KismetMaterialLibrary))
          (Rendering|Material|SetTextureParameterValue _returnvalue_2 "Texture" _returnvalue)
          (Rendering|Material|SetMaterial _waterpapersprite 0 _returnvalue_2)
          (Rendering|SetVisibility _waterpapersprite true false)
          (Variables|Default|SetWatermaskLoaded true))
        (:Is%20Not%20Valid
          (Variables|Default|SetWatermaskInvalid true))))))

(fn HideWatermask
  (Rendering|SetVisibility (Variables|Default|GetWaterPaperSprite) false false))

(fn RefreshWatermask
  (params (FilePath :type String) (TileSize :type Integer))
  (bind _returnvalue (Class|MyBlueprintFunctionLibrary|CreateTexturefromWatermaskArray FilePath TileSize))
  (Utilities|IsValid _returnvalue
    (:Is%20Valid
      (bind _returnvalue_2 (Rendering|Material|CreateDynamicMaterialInstance "/Game/Materials/M_BaseMaterial.M_BaseMaterial" "None" "Transient" :!class /Script/Engine.KismetMaterialLibrary))
      (Rendering|Material|SetTextureParameterValue _returnvalue_2 "Texture" _returnvalue)
      (Rendering|Material|SetMaterial (Variables|Default|GetWaterPaperSprite) 0 _returnvalue_2)
      (Variables|Default|SetWatermaskLoaded true))
    (:Is%20Not%20Valid
      (Variables|Default|SetWatermaskInvalid true))))