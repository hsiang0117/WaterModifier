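; Tile map manager that streams disk-based PNG map tiles as BP_Tile actors for the area under BP_Camera.
; On range changes it removes tiles outside the overlap and queues new ones; LOD changes rebuild the whole set, and both force garbage collection.
; A looping timer spawns one queued tile per firing and pauses when empty, spreading out load.
; It also shows, hides and refreshes per-tile water masks from .terrain files.
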(event EventBeginPlay
  (bind _returnvalue (Actor|GetActorOfClass "/Game/Blueprints/BP_Camera.BP_Camera_C"))
  (Variables|组件|SetCameraComponent (Actor|GetComponentbyClass _returnvalue "/Script/Engine.CameraComponent"))
  (bind _returnvalue_2 (Utilities|Time|SetTimerbyFunctionName 0 "Render" 0.01 true))
  (Variables|Default|SetMapTimerHandle _returnvalue_2))

(event Collision|EventActorBeginOverlap
  (params (OtherActor :type Actor%20Object%20Reference)))

(event EventTick
  (params (DeltaSeconds :type Float%20%28single-precision%29))
  (bind _returnvalue (Game|GetPlayerController 0))
  (bind _cameracomponent (Variables|组件|GetCameraComponent))
  (bind _asbp_my_player_controller (Utilities|Casting|CastToBP_MyPlayerController _returnvalue))
  (bind _currentlod (Variables|/Game/Blueprints/BP_MyPlayerController.BP_MyPlayerController_C|GetCurrentLod _asbp_my_player_controller))
  (bind _tilesize (Variables|/Game/Blueprints/BP_MyPlayerController.BP_MyPlayerController_C|GetTileSize _asbp_my_player_controller))
  (if (Variables|/Game/Blueprints/BP_MyPlayerController.BP_MyPlayerController_C|GetIsMapRootPathExist _asbp_my_player_controller)
    (Class|TileMapManager|Tick (Variables|组件|GetCameraComponent) _currentlod _tilesize
      (:OnRangeChange
        (bind _returnvalue_2 (Class|TileMapManager|GetBottomLeftandTopRight _cameracomponent _tilesize))
        (CallFunction|GetRenderListAfterRangeChanged (Variables|Default|GetLastTileIndex) _returnvalue_2 _currentlod)
        (Variables|Default|SetLastTileIndex _returnvalue_2))
      (:OnLodChange
        (bind _returnvalue_3 (Class|TileMapManager|GetBottomLeftandTopRight _cameracomponent _tilesize))
        (CallFunction|GetRenderListAfterLodChanged _returnvalue_3 _currentlod)
        (Variables|Default|SetLastTileIndex _returnvalue_3)))
    (Utilities|Platform|CollectGarbage)
    (Utilities|Time|UnpauseTimerbyHandle (Variables|Default|GetMapTimerHandle))))

(fn ConstructionScript)

(fn GetRenderListAfterLodChanged
  (params (TileIndex :type Int%20Vector%204%20Structure) (CurrentLod :type Integer))
  (bind _returnvalue (Game|GetPlayerController 0))
  (bind _tilelist (Variables|Default|GetTileList))
  (bind _asbp_my_player_controller (Utilities|Casting|CastToBP_MyPlayerController _returnvalue))
  (bind _tilestartnumber (Variables|/Game/Blueprints/BP_MyPlayerController.BP_MyPlayerController_C|GetTileStartNumber _asbp_my_player_controller))
  (bind _tilesize (Variables|/Game/Blueprints/BP_MyPlayerController.BP_MyPlayerController_C|GetTileSize _asbp_my_player_controller))
  (Utilities|Time|PauseTimerbyHandle (Variables|Default|GetMapTimerHandle))
  (for _array_element _tilelist
    (Actor|DestroyActor _array_element))
  (Utilities|Array|Clear _tilelist)
  (Utilities|Array|Clear (Variables|Default|GetTileToRender))
  (for _index (range (.x TileIndex) (.z TileIndex))
    (for _index_2 (range (.y TileIndex) (.w TileIndex))
      (bind _pngpath (CallFunction|ConstructPngPath CurrentLod (+ _index (.x _tilestartnumber)) (+ (.y _tilestartnumber) _index_2)))
      (if (Class|BlueprintPathsLibrary|FileExists _pngpath)
        (Utilities|Array|Add (Variables|Default|GetTileToRender) (Utilities|Struct|MakeTileToRender _pngpath (Math|Conversions|ToFloat(Integer) (* _tilesize _index)) (Math|Conversions|ToFloat(Integer) (* _tilesize _index_2)) (Utilities|Struct|MakeTileByIndex _index _index_2)))))))

(fn ConstructPngPath
  (params (CurrentLod :type Integer) (X :type Integer) (Y :type Integer))
  (return (Utilities|String|Append (Variables|/Game/Blueprints/BP_MyPlayerController.BP_MyPlayerController_C|GetMapRootPath (.AsBP%20My%20Player%20Controller (Utilities|Casting|CastToBP_MyPlayerController (Game|GetPlayerController 0)))) (Utilities|String|ToString(Integer) CurrentLod) "\\" (Utilities|String|ToString(Integer) X) "\\" (Utilities|String|ToString(Integer) Y) ".png")))

(fn GetRenderListAfterRangeChanged
  (params (LastTileIndex :type Int%20Vector%204%20Structure) (TileIndex :type Int%20Vector%204%20Structure) (CurrentLod :type Integer))
  (bind _returnvalue (Game|GetPlayerController 0))
  (bind _tiletorender (Variables|Default|GetTileToRender))
  (bind _tilelist (Variables|Default|GetTileList))
  (bind _asbp_my_player_controller (Utilities|Casting|CastToBP_MyPlayerController _returnvalue))
  (bind _tilesize (Variables|/Game/Blueprints/BP_MyPlayerController.BP_MyPlayerController_C|GetTileSize _asbp_my_player_controller))
  (bind _tilestartnumber (Variables|/Game/Blueprints/BP_MyPlayerController.BP_MyPlayerController_C|GetTileStartNumber _asbp_my_player_controller))
  (bind _returnvalue_2 (Class|TileMapManager|GetIntersection (Utilities|Struct|MakeIntPoint (.x LastTileIndex) (.y LastTileIndex)) (Utilities|Struct|MakeIntPoint (.z LastTileIndex) (.w LastTileIndex)) (Utilities|Struct|MakeIntPoint (.x TileIndex) (.y TileIndex)) (Utilities|Struct|MakeIntPoint (.z TileIndex) (.w TileIndex))))
  (Utilities|Time|PauseTimerbyHandle (Variables|Default|GetMapTimerHandle))
  (for _array_element _tilelist
    (if (not (Utilities|Array|ContainsItem _returnvalue_2 (Utilities|Struct|MakeIntPoint (Variables|/Game/Blueprints/BP_Tile.BP_Tile_C|GetX _array_element) (Variables|/Game/Blueprints/BP_Tile.BP_Tile_C|GetY _array_element))))
      (Actor|DestroyActor _array_element)
      (Utilities|Array|RemoveItem _tilelist _array_element)))
  (for (_array_element_2 _array_index) _tiletorender
    (if (not (Utilities|Array|ContainsItem _returnvalue_2 (Utilities|Struct|MakeIntPoint (.x (.tileindex _array_element_2)) (.y (.tileindex _array_element_2)))))
      (Utilities|Array|RemoveIndex _tiletorender _array_index)))
  (bind _returnvalue_3 (Class|TileMapManager|GetUnionMinusFirst (Utilities|Struct|MakeIntPoint (.x LastTileIndex) (.y LastTileIndex)) (Utilities|Struct|MakeIntPoint (.z LastTileIndex) (.w LastTileIndex)) (Utilities|Struct|MakeIntPoint (.x TileIndex) (.y TileIndex)) (Utilities|Struct|MakeIntPoint (.z TileIndex) (.w TileIndex))))
  (for _array_element_3 _returnvalue_3
    (bind _pngpath (CallFunction|ConstructPngPath CurrentLod (+ (.x _array_element_3) (.x _tilestartnumber)) (+ (.y _array_element_3) (.y _tilestartnumber))))
    (if (Class|BlueprintPathsLibrary|FileExists _pngpath)
      (Utilities|Array|Add (Variables|Default|GetTileToRender) (Utilities|Struct|MakeTileToRender _pngpath (Math|Conversions|ToFloat(Integer) (* (.x _array_element_3) _tilesize)) (Math|Conversions|ToFloat(Integer) (* (.y _array_element_3) _tilesize)) (Utilities|Struct|MakeTileByIndex (.x _array_element_3) (.y _array_element_3)))))))

(fn Render
  (bind _tiletorender (Variables|Default|GetTileToRender))
  (bind _output (Utilities|Array|Get(acopy) _tiletorender))
  (if (Utilities|Array|IsNotEmpty _tiletorender)
    (bind _array_element (Utilities|Array|ForEachLoopwithBreak (Variables|Default|GetTileList) :!label _label)
      (:LoopBody
        (if (and (== (Variables|/Game/Blueprints/BP_Tile.BP_Tile_C|GetX _array_element) (.x (.tileindex _output))) (== (Variables|/Game/Blueprints/BP_Tile.BP_Tile_C|GetY _array_element) (.y (.tileindex _output))))
          (LocalVariables|SetTileAlreadyExist true)
          (goto _label Break)))
      (:Completed
        (if (LocalVariables|GetTileAlreadyExist)
          _
          (else
            (bind _returnvalue (Game|SpawnActorfromClass "/Game/Blueprints/BP_Tile.BP_Tile_C" (Math|Transform|MakeTransform (Math|Vector|MakeVector (.loactionx _output) 0.0 (.loactiony _output)) "0, 0, 0" "1.000000,1.000000,1.000000") "Undefined" "MultiplyWithRoot" 0 0))
            (Variables|/Game/Blueprints/BP_Tile.BP_Tile_C|SetX _returnvalue (.x (.tileindex _output)))
            (Variables|/Game/Blueprints/BP_Tile.BP_Tile_C|SetY _returnvalue (.y (.tileindex _output)))
            (Default|SetTexture _returnvalue (.filepath _output))
            (Utilities|Array|Add (Variables|Default|GetTileList) _returnvalue)))
        (Utilities|Array|RemoveIndex (Variables|Default|GetTileToRender))))
    (else
      (Utilities|Time|PauseTimerbyHandle (Variables|Default|GetMapTimerHandle)))))

(fn ShowWatermask
  (bind _returnvalue (Game|GetPlayerController 0))
  (bind _asbp_my_player_controller (Utilities|Casting|CastToBP_MyPlayerController _returnvalue))
  (bind _tilestartnumber (Variables|/Game/Blueprints/BP_MyPlayerController.BP_MyPlayerController_C|GetTileStartNumber _asbp_my_player_controller))
  (for _array_element (Variables|Default|GetTileList)
    (Default|SetWatermask _array_element (Utilities|String|Append (Variables|/Game/Blueprints/BP_MyPlayerController.BP_MyPlayerController_C|GetTerrainRootPath _asbp_my_player_controller) (Utilities|String|ToString(Integer) (Variables|/Game/Blueprints/BP_MyPlayerController.BP_MyPlayerController_C|GetCurrentLod _asbp_my_player_controller)) "\\" (Utilities|String|ToString(Integer) (+ (Variables|/Game/Blueprints/BP_Tile.BP_Tile_C|GetX _array_element) (.x _tilestartnumber))) "\\" (Utilities|String|ToString(Integer) (+ (Variables|/Game/Blueprints/BP_Tile.BP_Tile_C|GetY _array_element) (.y _tilestartnumber))) ".terrain") (Variables|/Game/Blueprints/BP_MyPlayerController.BP_MyPlayerController_C|GetTileSize _asbp_my_player_controller))))

(fn HideWatermask
  (for _array_element (Variables|Default|GetTileList)
    (Default|HideWatermask _array_element)))

(fn RefreshWatermask
  (bind _returnvalue (Game|GetPlayerController 0))
  (bind _asbp_my_player_controller (Utilities|Casting|CastToBP_MyPlayerController _returnvalue))
  (bind _tilestartnumber (Variables|/Game/Blueprints/BP_MyPlayerController.BP_MyPlayerController_C|GetTileStartNumber _asbp_my_player_controller))
  (for _array_element (Variables|Default|GetTileList)
    (Default|RefreshWatermask _array_element (Utilities|String|Append (Variables|/Game/Blueprints/BP_MyPlayerController.BP_MyPlayerController_C|GetTerrainRootPath _asbp_my_player_controller) (Utilities|String|ToString(Integer) (Variables|/Game/Blueprints/BP_MyPlayerController.BP_MyPlayerController_C|GetCurrentLod _asbp_my_player_controller)) "\\" (Utilities|String|ToString(Integer) (+ (Variables|/Game/Blueprints/BP_Tile.BP_Tile_C|GetX _array_element) (.x _tilestartnumber))) "\\" (Utilities|String|ToString(Integer) (+ (Variables|/Game/Blueprints/BP_Tile.BP_Tile_C|GetY _array_element) (.y _tilestartnumber))) ".terrain") (Variables|/Game/Blueprints/BP_MyPlayerController.BP_MyPlayerController_C|GetTileSize _asbp_my_player_controller))))