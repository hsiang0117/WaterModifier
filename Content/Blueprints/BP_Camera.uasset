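; Orthographic camera for a tiled LOD map that pans in the X-Z plane by left-mouse drag, unless input is disabled or the click hits UI.
; Tick repositions it on LOD changes from stored coordinates, then writes current map coordinates back to BP_MyPlayerController.
; ClampLocation keeps the view within tile bounds after moves.
; BeginPlay matches the scene capture and render target size to the ortho width.
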(event Input|EnhancedActionEvents|EnhancedInputActionIA_LeftMouse
  (params (ActionValue :type Boolean) (ElapsedSeconds :type Float%20%28double-precision%29) (TriggeredSeconds :type Float%20%28double-precision%29) (InputAction :type Input%20Action%20Object%20Reference :default "/Game/Input/IA_LeftMouse.IA_LeftMouse"))
  (bind _returnvalue (Game|GetPlayerController 0))
  (bind _returnvalue_2 (Game|GetPlayerController 0))
  (bind _camera (Variables|Default|GetCamera))
  (bind (_sizex _sizey) (HUD|GetViewportSize _returnvalue))
  (bind (_locationx _locationy) (Game|Player|GetMousePosition _returnvalue))
  (bind _asbp_my_player_controller (Utilities|Casting|CastToBP_MyPlayerController _returnvalue_2))
  (bind _orthowidth (Variables|/Script/Engine.CameraComponent|GetOrthoWidth _camera))
  (bind _isclickonui (Variables|/Game/Blueprints/BP_MyPlayerController.BP_MyPlayerController_C|GetIsClickOnUI _asbp_my_player_controller))
  (bind _isinputdisabled (Variables|/Game/Blueprints/BP_MyPlayerController.BP_MyPlayerController_C|GetIsInputDisabled _asbp_my_player_controller))
  (:Triggered
    (if (not _isinputdisabled)
      (if (not _isclickonui)
        (bind _output_get (Variables|Default|SetNow (Math|Vector2D|MakeVector2D _locationx _locationy)))
        (Transformation|AddActorWorldOffset (Math|Vector|MakeVector (* (/ (- (.x (stale _output_get_2)) (.x _output_get)) _sizex) _orthowidth) 0.0 (* (/ (- (.y _output_get) (.y (stale _output_get_2))) _sizey) _orthowidth)))
        (CallFunction|ClampLocation)
        (Variables|Default|SetOrigin (Variables|Default|GetNow))
        (Variables|/Script/Engine.PlayerController|SetCurrentMouseCursor _returnvalue "GrabHand"))))
  (:Started
    (if (not _isinputdisabled)
      (if (not _isclickonui)
        (bind _output_get_2 (Variables|Default|SetOrigin (Math|Vector2D|MakeVector2D _locationx _locationy))))))
  (:Completed
    (if (not _isinputdisabled)
      (if (not _isclickonui)
        (Variables|/Script/Engine.PlayerController|SetCurrentMouseCursor _returnvalue "Default")))))

(event EventBeginPlay
  (Variables|/Script/Engine.SceneCaptureComponent2D|SetOrthoWidth (Variables|Default|GetSceneCaptureComponent2D) (Variables|/Script/Engine.CameraComponent|GetOrthoWidth (Variables|Default|GetCamera)))
  (Rendering|ResizeRenderTarget2D "/Game/Textures/RT_RenderTarget.RT_RenderTarget" (Math|Float|Truncate (Variables|/Script/Engine.CameraComponent|GetOrthoWidth (Variables|Default|GetCamera))) (Math|Float|Truncate (Variables|/Script/Engine.CameraComponent|GetOrthoWidth (Variables|Default|GetCamera)))))

(event Collision|EventActorBeginOverlap
  (params (OtherActor :type Actor%20Object%20Reference)))

(event EventTick
  (params (DeltaSeconds :type Float%20%28single-precision%29))
  (bind _returnvalue (Game|GetPlayerController 0))
  (bind _asbp_my_player_controller (Utilities|Casting|CastToBP_MyPlayerController _returnvalue))
  (bind _ismaprootpathexist (Variables|/Game/Blueprints/BP_MyPlayerController.BP_MyPlayerController_C|GetIsMapRootPathExist _asbp_my_player_controller))
  (bind _currentlod (Variables|/Game/Blueprints/BP_MyPlayerController.BP_MyPlayerController_C|GetCurrentLod _asbp_my_player_controller))
  (bind _unitslist (Variables|/Game/Blueprints/BP_MyPlayerController.BP_MyPlayerController_C|GetUnitsList _asbp_my_player_controller))
  (bind _tilestartnumber (Variables|/Game/Blueprints/BP_MyPlayerController.BP_MyPlayerController_C|GetTileStartNumber _asbp_my_player_controller))
  (bind _tilesize (Variables|/Game/Blueprints/BP_MyPlayerController.BP_MyPlayerController_C|GetTileSize _asbp_my_player_controller))
  (Utilities|FlowControl|Sequence
    (:then_0
      (if _ismaprootpathexist
        (bind _returnvalue_2 (Class|MyBlueprintFunctionLibrary|IsLodChanged _currentlod))
        (if _returnvalue_2
          (bind _returnvalue_3 (Class|MyBlueprintFunctionLibrary|GetNewPositionAfterLodChange _currentlod _tilesize (Variables|/Game/Blueprints/BP_MyPlayerController.BP_MyPlayerController_C|GetCameraCoordinates _asbp_my_player_controller) _unitslist _tilestartnumber))
          (Transformation|SetActorLocation (Math|Vector|MakeVector (.x _returnvalue_3) 1e+02 (.y _returnvalue_3)) false false)
          (CallFunction|ClampLocation))))
    (:then_1
      (if _ismaprootpathexist
        (bind _returnvalue_4 (Class|MyBlueprintFunctionLibrary|GetCurrentCameraCoordinates (Transformation|GetActorLocation) _tilestartnumber _tilesize _currentlod _unitslist))
        (Variables|/Game/Blueprints/BP_MyPlayerController.BP_MyPlayerController_C|SetCameraCoordinates _asbp_my_player_controller (Math|Vector2D|MakeVector2D (.x _returnvalue_4) (.y _returnvalue_4)))))))

(fn ConstructionScript)

(fn ClampLocation
  (bind _returnvalue (Transformation|GetActorLocation))
  (bind _returnvalue_2 (Game|GetPlayerController 0))
  (bind _camera (Variables|Default|GetCamera))
  (bind _asbp_my_player_controller (Utilities|Casting|CastToBP_MyPlayerController _returnvalue_2))
  (bind _orthowidth (Variables|/Script/Engine.CameraComponent|GetOrthoWidth _camera))
  (bind _returnvalue_3 (/ _orthowidth 2.0))
  (bind _tilenumbers (Variables|/Game/Blueprints/BP_MyPlayerController.BP_MyPlayerController_C|GetTileNumbers _asbp_my_player_controller))
  (bind _tilesize (Variables|/Game/Blueprints/BP_MyPlayerController.BP_MyPlayerController_C|GetTileSize _asbp_my_player_controller))
  (Transformation|SetActorLocation (Math|Vector|MakeVector (Math|Float|Clamp(Float) (.x _returnvalue) _returnvalue_3 (- (Math|Conversions|ToFloat(Integer) (* (.x _tilenumbers) _tilesize)) _returnvalue_3)) (.y _returnvalue) (Math|Float|Clamp(Float) (.z _returnvalue) _returnvalue_3 (- (Math|Conversions|ToFloat(Integer) (* (.y _tilenumbers) _tilesize)) _returnvalue_3))) false false))