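; Actor that keeps a TCP client connection to a local server on a hardcoded port, reconnecting on disconnect.
; On connect it enables touch and input mapping, fires Connected, and sends the camera's ortho width as length-prefixed messages.
; Incoming "Done" strings for Set Image, Modify and Segment trigger matching calls; other messages set NumModified on the player controller.
; It reads port.txt but leaves the value unused.
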(event Custom|OnDisconnected
  (params (ConnectionId :type Integer))
  (bind _connectionid (Class|TcpSocketConnection|Connect "127.0.0.1" 10086 (delegate Custom|OnDisconnected) (delegate Custom|OnConnected) (delegate Custom|OnMessageReceived)))
  (Variables|Default|SetConnectionId _connectionid))

(event Custom|OnConnected
  (params (ConnectionId :type Integer))
  (bind _returnvalue (Game|GetPlayerController 0))
  (bind _returnvalue_2 (PlayerController|LocalPlayerSubsystems|GetEnhancedInputLocalPlayerSubsystem _returnvalue))
  (Variables|/Script/Engine.PlayerController|SetbEnableTouchEvents _returnvalue true)
  (Utilities|IsValid _returnvalue_2
    (:Is%20Valid
      (Input|AddMappingContext _returnvalue_2 "/Game/Input/InputMapping.InputMapping" 0 "(bIgnoreAllPressedKeysUntilRelease=True,bForceImmediately=False,bNotifyUserSettings=False)")
      (Default|CallConnected)
      (CallFunction|SendMessage "OrthoWidth")
      (bind _returnvalue_3 (Actor|GetActorOfClass "/Game/Blueprints/BP_Camera.BP_Camera_C"))
      (CallFunction|SendMessage (Utilities|String|ToString(Integer) (Math|Float|Truncate (Variables|/Script/Engine.CameraComponent|GetOrthoWidth (Actor|GetComponentbyClass _returnvalue_3 "/Script/Engine.CameraComponent"))))))))

(event Custom|OnMessageReceived
  (params (ConnectionId :type Integer) (Message :type Array%20of%20Bytes))
  (bind _returnvalue (Class|TcpSocketConnection|MessageReadString Message (Utilities|Array|Length Message)))
  (switch string _returnvalue
    (:Default
      (Variables|/Game/Blueprints/BP_MyPlayerController.BP_MyPlayerController_C|SetNumModified (.AsBP%20My%20Player%20Controller (Utilities|Casting|CastToBP_MyPlayerController (Game|GetPlayerController 0))) _returnvalue))
    (:SetImageDone
      (Default|CallSetImageDone))
    (:ModifyDone
      (Default|CallModifyDone))
    (:SegmentDone
      (Default|CallSegmentDone))))

(event EventEndPlay
  (params (EndPlayReason :type EEndPlayReason%20Enum :default "Destroyed"))
  (Class|TcpSocketConnection|Disconnect (stale Custom|OnDisconnected _connectionid)))

(event Collision|EventActorBeginOverlap
  (params (OtherActor :type Actor%20Object%20Reference)))

(event EventTick
  (params (DeltaSeconds :type Float%20%28single-precision%29)))

(event EventBeginPlay
  (bind _outcontent (Class|MyBlueprintFunctionLibrary|ReadFile "port.txt"))
  (bind _connectionid (Class|TcpSocketConnection|Connect "127.0.0.1" 10086 (delegate Custom|OnDisconnected) (delegate Custom|OnConnected) (delegate Custom|OnMessageReceived)))
  (Variables|Default|SetConnectionId _connectionid))

(fn ConstructionScript)

(fn SendMessage
  (params (Message :type String))
  (bind _returnvalue (Class|TcpSocketConnection|ToBytes(String) Message))
  (bind _connectionid (Variables|Default|GetConnectionId))
  (bind _returnvalue_2 (Class|TcpSocketConnection|SendData _connectionid (Class|TcpSocketConnection|ToBytes(Integer) (Utilities|Array|Length _returnvalue))))
  (bind _returnvalue_3 (Class|TcpSocketConnection|SendData _connectionid _returnvalue))
  (return (and _returnvalue_3 _returnvalue_2)))