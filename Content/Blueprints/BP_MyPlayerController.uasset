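; BP_MyPlayerController is a player controller that creates the main user interface and relays TCP socket results to it.
; On BeginPlay it shows the mouse cursor, adds the UserInterface widget to the viewport and finds the BP_TCPSocketConnection actor in the level.
; It binds that actor's SegmentDone, SetImageDone, ModifyDone and Connected events, forwarding each to the matching handler on the widget.
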(event Custom|SetImageDone_事件
  (Default|OnSetImageDone (stale EventBeginPlay _output_get)))

(event Custom|SegmentDone_事件
  (Default|OnSegmentDone (stale EventBeginPlay _output_get)))

(event Custom|Connected_事件
  (Default|OnConnected (stale EventBeginPlay _output_get)))

(event Custom|ModifyDone_事件
  (Default|OnModifyDone (stale EventBeginPlay _output_get)))

(event EventBeginPlay
  (Variables|Default|SetbShowMouseCursor self true)
  (bind _returnvalue (UserInterface|CreateWidget "/Game/UI/UserInterface.UserInterface_C"))
  (bind _output_get (Variables|Default|SetUserInterface _returnvalue))
  (UserInterface|Viewport|AddtoViewport _output_get 0)
  (bind _returnvalue_2 (Actor|GetActorOfClass "/Game/Blueprints/BP_TCPSocketConnection.BP_TCPSocketConnection_C"))
  (EventDispatchers|AssignSegmentDone _returnvalue_2 (delegate Custom|SegmentDone_事件))
  (EventDispatchers|AssignSetImageDone _returnvalue_2 (delegate Custom|SetImageDone_事件))
  (EventDispatchers|BindEventtoModifyDone _returnvalue_2 (delegate Custom|ModifyDone_事件))
  (EventDispatchers|BindEventtoConnected _returnvalue_2 (delegate Custom|Connected_事件)))

(event EventTick
  (params (DeltaSeconds :type Float%20%28single-precision%29)))

(fn ConstructionScript)