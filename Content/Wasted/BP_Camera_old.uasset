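; Orthographic camera pawn that shows a pannable, zoomable 2D tiled map built from PNG tiles on disk.
; Left-drag pans by deprojected mouse delta; scroll halves or doubles ortho width and steps LodLevel, clamping to map bounds when zooming out.
; Visible tile indices come from camera position and width; Render destroys all tiles, then respawns BP_Tile_old sprites with textures imported by zoom/X/flipped-Y path.
; Input is ignored while the player controller is operating UI.
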(event Custom|Render
  (bind _lodlevel (Variables|Default|GetLodLevel))
  (bind _tilelist (Variables|Default|GetTileList))
  (bind _returnvalue (Math|Float|Power 2.0 _lodlevel))
  (bind _returnvalue_2 (- 9.0 _lodlevel))
  (bind _returnvalue_3 (Math|Float|Truncate _returnvalue_2))
  (for _array_element _tilelist
    (Actor|DestroyActor _array_element))
  (Utilities|Array|Clear _tilelist)
  (for _index (range (Variables|Default|GetTopLeftX) (Variables|Default|GetBottomRightX))
    (for _index_2 (range (Variables|Default|GetTopLeftY) (Variables|Default|GetBottomRightY))
      (bind _returnvalue_4 (Game|SpawnActorfromClass "/Game/Wasted/BP_Tile_old.BP_Tile_old_C" (Math|Transform|MakeTransform (Math|Vector|MakeVector (* _index 256 _returnvalue) 0.0 (* _index_2 -256 _returnvalue)) "0, 0, 0" (Math|Vector|MakeVector _returnvalue 1.0 _returnvalue)) "Undefined" "MultiplyWithRoot" 0 0))
      (bind _returnvalue_5 (Class|MyBlueprintFunctionLibrary|MyImportFileasTexture2D (Utilities|String|Append (Variables|Default|GetFilePath) (Utilities|String|ToString(Integer) _returnvalue_3) "/" (Utilities|String|ToString(Integer) _index) "/" (Utilities|String|ToString(Integer) (Math|Float|Truncate (Utilities|Operators|Subtract (Math|Float|Power 2.0 (Math|Conversions|ToFloat(Integer) _returnvalue_3)) 1.0 _index_2))) ".png")))
      (Utilities|IsValid _returnvalue_5
        (:Is%20Valid
          (Variables|/Script/Engine.Texture|SetCompressionSettings _returnvalue_5 "TC_EditorIcon")
          (Variables|/Script/Engine.Texture|SetLODGroup _returnvalue_5 "TEXTUREGROUP_Pixels2D")
          (bind _returnvalue_6 (Rendering|Material|CreateDynamicMaterialInstance (Variables|/Game/Wasted/BP_Tile_old.BP_Tile_old_C|GetPaperSprite _returnvalue_4) 0 "/Game/Materials/M_BaseMaterial.M_BaseMaterial" "None" :!class /Script/Engine.PrimitiveComponent))
          (Rendering|Material|SetTextureParameterValue _returnvalue_6 "Texture" _returnvalue_5)
          (Utilities|Array|Add (Variables|Default|GetTileList) _returnvalue_4))
        (:Is%20Not%20Valid
          (Actor|DestroyActor _returnvalue_4))))))

(event Custom|GetTopLeftAndBottomRightPos
  (bind _self self)
  (bind _camera (Variables|Default|GetCamera))
  (bind _lodlevel (Variables|Default|GetLodLevel))
  (bind _returnvalue (Transformation|GetActorLocation _self))
  (bind _returnvalue_2 (Math|Float|Power 2.0 _lodlevel))
  (bind _orthowidth (Variables|/Script/Engine.CameraComponent|GetOrthoWidth _camera))
  (bind _returnvalue_3 (/ _orthowidth 2.0))
  (bind _returnvalue_4 (/ _orthowidth 4.0))
  (bind _returnvalue_5 (* 256 _returnvalue_2))
  (bind _returnvalue_6 (+ (.x _returnvalue) _returnvalue_3))
  (bind _returnvalue_7 (- (.z _returnvalue) _returnvalue_4))
  (bind _returnvalue_8 (Class|KismetMathLibrary|ToInt64(Float) _returnvalue_6))
  (bind _returnvalue_9 (Class|KismetMathLibrary|ToInt64(Float) _returnvalue_7))
  (bind _returnvalue_10 (Math|Conversions|ToInteger(Byte) _returnvalue_8))
  (bind _returnvalue_11 (Math|Conversions|ToInteger(Byte) _returnvalue_9))
  (bind _returnvalue_12 (/ _returnvalue_11 _returnvalue_5))
  (bind _returnvalue_13 (/ _returnvalue_10 _returnvalue_5))
  (Variables|Default|SetTopLeftX (/ (Math|Conversions|ToInteger(Byte) (Class|KismetMathLibrary|ToInt64(Float) (- (.x _returnvalue) _returnvalue_3))) _returnvalue_5))
  (Variables|Default|SetTopLeftY (Utilities|Operators|Divide (Math|Conversions|ToInteger(Byte) (Class|KismetMathLibrary|ToInt64(Float) (+ (.z _returnvalue) _returnvalue_4))) _returnvalue_5 -1))
  (if (!= (Math|Integer|%(Integer) _returnvalue_10 _returnvalue_5) 0)
    (Variables|Default|SetBottomRightX _returnvalue_13)
    (else
      (Variables|Default|SetBottomRightX (- _returnvalue_13 1))))
  (if (!= (Math|Integer|%(Integer) _returnvalue_11 _returnvalue_5) 0)
    (Variables|Default|SetBottomRightY (- 0 _returnvalue_12))
    (else
      (Variables|Default|SetBottomRightY (- 0 (+ _returnvalue_12 1))))))

(event Input|EnhancedActionEvents|EnhancedInputActionIA_LeftMouse
  (params (ActionValue :type Boolean) (ElapsedSeconds :type Float%20%28double-precision%29) (TriggeredSeconds :type Float%20%28double-precision%29) (InputAction :type Input%20Action%20Object%20Reference :default "/Game/Input/IA_LeftMouse.IA_LeftMouse"))
  (bind _returnvalue (Game|GetPlayerController 0))
  (bind _returnvalue_2 (Game|GetPlayerController 0))
  (bind _worldlocation (Game|Player|ConvertMouseLocationToWorldSpace _returnvalue))
  (bind _asbp_my_player_controller (Utilities|Casting|CastToBP_MyPlayerController _returnvalue_2))
  (bind _isoperatingui (Variables|/Game/Blueprints/BP_MyPlayerController.BP_MyPlayerController_C|GetIsOperatingUI _asbp_my_player_controller))
  (:Triggered
    (if (not _isoperatingui)
      (bind _output_get (Variables|Default|SetNow _worldlocation))
      (Transformation|AddActorWorldOffset (- _output_get (stale _output_get_2)))
      (Variables|Default|SetOrigin (Variables|Default|GetNow))
      (Variables|/Script/Engine.PlayerController|SetCurrentMouseCursor _returnvalue "GrabHand")
      (CallFunction|GetTopLeftandBottomRightPos)
      (if (not (Math|Boolean|ANDBoolean (== (Variables|Default|GetOldTopLeftX) (Variables|Default|GetTopLeftX)) (== (Variables|Default|GetTopLeftY) (Variables|Default|GetOldTopLeftY)) (== (Variables|Default|GetBottomRightX) (Variables|Default|GetOldBottomRightX)) (== (Variables|Default|GetBottomRightY) (Variables|Default|GetOldBottomRightY))))
        (Variables|Default|SetOldTopLeftX (Variables|Default|GetTopLeftX))
        (Variables|Default|SetOldTopLeftY (Variables|Default|GetTopLeftY))
        (Variables|Default|SetOldBottomRightX (Variables|Default|GetBottomRightX))
        (Variables|Default|SetOldBottomRightY (Variables|Default|GetBottomRightY))
        (CallFunction|Render))))
  (:Started
    (if (not _isoperatingui)
      (bind _output_get_2 (Variables|Default|SetOrigin _worldlocation))))
  (:Completed
    (if (not _isoperatingui)
      (Variables|/Script/Engine.PlayerController|SetCurrentMouseCursor _returnvalue "Default"))))

(event Input|EnhancedActionEvents|EnhancedInputActionIA_Scroll
  (params (ActionValue :type Float%20%28double-precision%29) (ElapsedSeconds :type Float%20%28double-precision%29) (TriggeredSeconds :type Float%20%28double-precision%29) (InputAction :type Input%20Action%20Object%20Reference :default "/Game/Input/IA_Scroll.IA_Scroll"))
  (bind _self self)
  (bind _self_2 self)
  (bind _self_3 self)
  (bind _self_4 self)
  (bind _self_5 self)
  (bind _self_6 self)
  (bind _lodlevel (Variables|Default|GetLodLevel))
  (bind _lodlevel_2 (Variables|Default|GetLodLevel))
  (bind _camera (Variables|Default|GetCamera))
  (bind _returnvalue (Transformation|GetActorLocation _self))
  (bind _returnvalue_2 (Transformation|GetActorLocation _self_4))
  (bind _returnvalue_3 (Transformation|GetActorLocation _self_5))
  (bind _returnvalue_4 (Transformation|GetActorLocation _self_6))
  (bind _returnvalue_5 (Transformation|GetActorLocation _self_2))
  (bind _returnvalue_6 (Transformation|GetActorLocation _self_3))
  (:Started
    (if (not (Variables|/Game/Blueprints/BP_MyPlayerController.BP_MyPlayerController_C|GetIsOperatingUI (.AsBP%20My%20Player%20Controller (Utilities|Casting|CastToBP_MyPlayerController (Game|GetPlayerController 0)))))
      (if (> ActionValue 0.0)
        (if (> _lodlevel 0.0)
          (Variables|/Script/Engine.SceneCaptureComponent2D|SetOrthoWidth (Variables|Default|GetSceneCaptureComponent2D) (/ (Variables|/Script/Engine.CameraComponent|GetOrthoWidth _camera) 2.0))
          (Class|CameraComponent|SetOrthoWidth _camera (/ (Variables|/Script/Engine.CameraComponent|GetOrthoWidth _camera) 2.0))
          (Variables|Default|SetSpeed (/ (Variables|Default|GetSpeed) 2.0))
          (Math|Float|DecrementFloat _lodlevel_2
            (:%20%20
              (CallFunction|GetTopLeftandBottomRightPos :!label _label)
              (CallFunction|Render))))
        (elif (< _lodlevel 9.0)
          (Variables|/Script/Engine.SceneCaptureComponent2D|SetOrthoWidth (Variables|Default|GetSceneCaptureComponent2D) (* (Variables|/Script/Engine.CameraComponent|GetOrthoWidth _camera) 2.0))
          (Class|CameraComponent|SetOrthoWidth _camera (* (Variables|/Script/Engine.CameraComponent|GetOrthoWidth _camera) 2.0))
          (Variables|Default|SetSpeed (* (Variables|Default|GetSpeed) 2.0))
          (Math|Float|IncrementFloat _lodlevel_2
            (:%20%20
              (Utilities|FlowControl|Sequence
                (:then_0
                  (if (< (- (.x _returnvalue_4) (/ (Variables|/Script/Engine.CameraComponent|GetOrthoWidth (Variables|Default|GetCamera)) 2.0)) 0.0)
                    (Transformation|SetActorLocation _self_5 (Math|Vector|MakeVector (/ (Variables|/Script/Engine.CameraComponent|GetOrthoWidth (Variables|Default|GetCamera)) 2.0) (.y _returnvalue_3) (.z _returnvalue_3)) false false)
                    (goto _label)
                    (else
                      (goto _label))))
                (:then_1
                  (if (> (+ (.x _returnvalue_4) (/ (Variables|/Script/Engine.CameraComponent|GetOrthoWidth (Variables|Default|GetCamera)) 2.0)) (* (Math|Float|Power 2.0 9.0) (Variables|Default|GetTileSize) 2.0))
                    (Transformation|SetActorLocation _self_2 (Math|Vector|MakeVector (- (* (Math|Float|Power 2.0 9.0) (Variables|Default|GetTileSize) 2.0) (/ (Variables|/Script/Engine.CameraComponent|GetOrthoWidth (Variables|Default|GetCamera)) 2.0)) (.y _returnvalue_5) (.z _returnvalue_5)) false false)
                    (goto _label)
                    (else
                      (goto _label))))
                (:then_2
                  (if (> (+ (.z _returnvalue) (/ (Variables|/Script/Engine.CameraComponent|GetOrthoWidth (Variables|Default|GetCamera)) 4.0)) 0.0)
                    (Transformation|SetActorLocation _self_3 (Math|Vector|MakeVector (.x _returnvalue_6) (.y _returnvalue_6) (/ (Variables|/Script/Engine.CameraComponent|GetOrthoWidth (Variables|Default|GetCamera)) -4.0)) false false)
                    (goto _label)
                    (else
                      (goto _label))))
                (:then_3
                  (if (< (- (.z _returnvalue) (/ (Variables|/Script/Engine.CameraComponent|GetOrthoWidth (Variables|Default|GetCamera)) 4.0)) (* (Math|Float|Power 2.0 9.0) (Variables|Default|GetTileSize) -1.0))
                    (Transformation|SetActorLocation _self_4 (Math|Vector|MakeVector (.x _returnvalue_2) (.y _returnvalue_2) (+ (/ (Variables|/Script/Engine.CameraComponent|GetOrthoWidth (Variables|Default|GetCamera)) 4.0) (* (Math|Float|Power 2.0 9.0) (Variables|Default|GetTileSize) -1.0))) false false)
                    (goto _label)
                    (else
                      (goto _label))))))))))))

(event EventBeginPlay
  (bind _lodlevel (Variables|Default|GetLodLevel))
  (bind _tilesize (Variables|Default|GetTileSize))
  (bind _returnvalue (Math|Float|Power 2.0 _lodlevel))
  (bind _returnvalue_2 (* _tilesize _returnvalue 2.0))
  (bind _returnvalue_3 (* _tilesize _returnvalue))
  (bind _as玩家控制器 (Utilities|Casting|CastToPlayerController (Pawn|GetController)))
  (Variables|/Script/Engine.PlayerController|SetbShowMouseCursor _as玩家控制器 true)
  (Variables|/Script/Engine.PlayerController|SetbEnableTouchEvents _as玩家控制器 true)
  (Utilities|IsValid (PlayerController|LocalPlayerSubsystems|GetEnhancedInputLocalPlayerSubsystem _as玩家控制器)
    (:Is%20Valid
      (Input|AddMappingContext (PlayerController|LocalPlayerSubsystems|GetEnhancedInputLocalPlayerSubsystem _as玩家控制器) "/Game/Input/InputMapping.InputMapping" 0 "(bIgnoreAllPressedKeysUntilRelease=True,bForceImmediately=False,bNotifyUserSettings=False)")
      (Variables|/Script/Engine.SceneCaptureComponent2D|SetOrthoWidth (Variables|Default|GetSceneCaptureComponent2D) _returnvalue_2)
      (Class|CameraComponent|SetOrthoWidth (Variables|Default|GetCamera) _returnvalue_2)
      (Transformation|SetActorLocation (Math|Vector|MakeVector _returnvalue_3 1e+02 (* _returnvalue_3 -0.5)) false false)
      (Transformation|SetActorRotation "0.000000,-90.000000,0.000000")
      (CallFunction|GetTopLeftandBottomRightPos)
      (CallFunction|Render))))

(event Collision|EventActorBeginOverlap
  (params (OtherActor :type Actor%20Object%20Reference)))

(event EventTick
  (params (DeltaSeconds :type Float%20%28single-precision%29)))

(fn ConstructionScript)